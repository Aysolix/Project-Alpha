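; Base puzzle console actor that switches the player between gameplay and a puzzle interface.
; Opening attaches the passed-in player camera to PuzzleView, sets UI-only input focused on InterfaceWidget with a visible cursor, and removes the Interactable tag.
; Closing reattaches the camera to its saved boom, restores game input and re-adds the tag.
; BackLight events give console feedback with a brief red flash or a lasting green.
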(event Custom|SetUIInputMode
  (bind _returnvalue (Game|GetPlayerController 0))
  (Input|SetInputModeUIOnly _returnvalue (UserInterface|GetUserWidgetObject (Variables|Default|GetInterfaceWidget)) "LockAlways" false)
  (Variables|/Script/Engine.PlayerController|SetbShowMouseCursor _returnvalue true))

(event Custom|SetGameInputMode
  (bind _returnvalue (Game|GetPlayerController 0))
  (Input|SetInputModeGameOnly _returnvalue false)
  (Variables|/Script/Engine.PlayerController|SetbShowMouseCursor _returnvalue false))

(event Custom|SetConsoleGreen
  (Rendering|Components|Light|SetLightColor (Variables|Default|GetBackLight) "(R=0.000000,G=1.000000,B=0.000000,A=1.000000)" true))

(event Custom|FlashConsoleRed
  (Rendering|Components|Light|SetLightColor (Variables|Default|GetBackLight) "(R=1.000000,G=0.000000,B=0.000000,A=1.000000)" true)
  (Utilities|FlowControl|Delay 1.0)
  (Rendering|Components|Light|SetLightColor (Variables|Default|GetBackLight) "(R=1.000000,G=1.000000,B=1.000000,A=1.000000)" true))

(fn ConstructionScript)

(fn OpenPuzzleInterface
  (params (Camera :type Camera%20Component%20Object%20Reference) (CameraBoom :type Spring%20Arm%20Component%20Object%20Reference))
  (Variables|Default|SetMainCameraBoom CameraBoom)
  (bind _output_get (Variables|Default|SetMainCamera Camera))
  (Transformation|AttachComponentToComponent _output_get (Variables|Default|GetPuzzleView) "None" "KeepRelative" "KeepRelative" "KeepRelative" true)
  (CallFunction|SetUIInputMode)
  (Utilities|Array|RemoveItem (Variables|Actor|GetTags) "Interactable"))

(fn ClosePuzzleInterface
  (Transformation|AttachComponentToComponent (Variables|Default|GetMainCamera) (Variables|Default|GetMainCameraBoom) "None" "KeepRelative" "KeepRelative" "KeepRelative" true)
  (CallFunction|SetGameInputMode)
  (Utilities|Array|Add (Variables|Actor|GetTags) "Interactable"))
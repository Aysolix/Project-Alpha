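; Number puzzle key that generates a random four-digit code and displays it.
; GenerateKey calls the ServerGenerateKey event, which joins four random digits from 0 to 8 into the Key string, then returns Key.
; The OnRep notify for Key writes the code to KeyText.
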(event Custom|ServerGenerateKey
  (Variables|Default|SetKey (Utilities|String|Append (Utilities|String|ToString(Integer) (Math|Random|RandomInteger 9)) (Utilities|String|ToString(Integer) (Math|Random|RandomInteger 9)) (Utilities|String|ToString(Integer) (Math|Random|RandomInteger 9)) (Utilities|String|ToString(Integer) (Math|Random|RandomInteger 9)))))

(fn ConstructionScript)

(fn GenerateKey
  (CallFunction|ServerGenerateKey)
  (return (Variables|Default|GetKey)))

(fn OnRepKey
  (Rendering|Components|TextRender|SetText (Variables|Default|GetKeyText) (Utilities|Text|ToText(String) (Variables|Default|GetKey))))
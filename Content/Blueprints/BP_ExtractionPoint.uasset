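; Extraction point that removes BP_Cargo actors inside its box and counts down the cargo still required.
; ExtractCargo starts a run unless one is active; after a delay, overlapping cargo is destroyed and the WB_ExtractionNumber widget count updates.
; A colored light signals working, success or empty box.
; After a success, it prints completion at zero remaining or re-runs itself if more cargo overlaps.
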(event Custom|RunExtractCargo
  (bind _box (Variables|Default|GetBox))
  (bind _extractionlight (Variables|Default|GetExtractionLight))
  (bind _overlappingactors (Collision|GetOverlappingActors _box "/Game/Blueprints/BP_Cargo.BP_Cargo_C" :!class /Script/Engine.PrimitiveComponent))
  (if (> (Variables|Default|GetCargoRemaining) 0)
    (Variables|Default|SetIsExtracting true)
    (Rendering|SetVisibility (Variables|Default|GetExtractionLight) true false)
    (Rendering|Components|Light|SetLightColor (Variables|Default|GetExtractionLight) "(R=1.000000,G=1.000000,B=0.000000,A=1.000000)" true)
    (CallFunction|UpdateNumber (Variables|Default|GetCargoRemaining))
    (Utilities|FlowControl|Delay 2.0)
    (if (> (Utilities|Array|Length _overlappingactors) 0)
      (for _array_element _overlappingactors
        (bind _output_get (Variables|Default|SetCargoRemaining (- (Variables|Default|GetCargoRemaining) 1)))
        (CallFunction|UpdateNumber _output_get)
        (Actor|DestroyActor _array_element)
        (Rendering|Components|Light|SetLightColor (Variables|Default|GetExtractionLight) "(R=0.000000,G=1.000000,B=0.000000,A=1.000000)" true)
        (Utilities|FlowControl|Delay 1.0)
        (Rendering|SetVisibility (Variables|Default|GetExtractionLight) false false)
        (Variables|Default|SetIsExtracting false)
        (if (== _output_get 0)
          (Development|PrintString "Extraction Complete!")
          (elif (> (Utilities|Array|Length (Collision|GetOverlappingActors (Variables|Default|GetBox) "/Game/Blueprints/BP_Cargo.BP_Cargo_C" :!class /Script/Engine.PrimitiveComponent)) 0)
            (CallFunction|RunExtractCargo))))
      (else
        (Rendering|Components|Light|SetLightColor _extractionlight "(R=1.000000,G=0.000000,B=0.000000,A=1.000000)" true)
        (Utilities|FlowControl|Delay 1.0)
        (Rendering|SetVisibility _extractionlight false false)
        (Variables|Default|SetIsExtracting false)))))

(fn ConstructionScript)

(fn ExtractCargo
  (if (not (Variables|Default|GetIsExtracting))
    (CallFunction|RunExtractCargo)))

(fn UpdateNumber
  (params (CargoRemaining :type Integer))
  (bind _aswb_extraction_number (Utilities|Casting|CastToWB_ExtractionNumber (UserInterface|GetUserWidgetObject (Variables|Default|GetInterfaceWidget))))
  (Default|UpdateNumberTextBox _aswb_extraction_number CargoRemaining))
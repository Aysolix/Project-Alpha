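; BP_Door is a door that stays locked until BP_BatteryStorage holds enough collected batteries.
; OpenCloseDoor plays a low-pitched click while locked; once unlocked, a FlipFlop alternates opening and closing with matching sounds.
; One timeline plays forward or in reverse to swing the door's yaw through 90 degrees.
; CheckUpdateBatteryColour changes the VaultBattery light colour when the same battery threshold is met.
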(event Custom|OpenCloseDoor
  (bind _returnvalue (Actor|GetActorOfClass "/Game/Blueprints/BP_BatteryStorage.BP_BatteryStorage_C"))
  (if (< (Variables|/Game/Blueprints/BP_BatteryStorage.BP_BatteryStorage_C|GetBatteriesCollected _returnvalue) (Variables|Default|GetBatteriesRequiredToUnlock))
    (Audio|PlaySound2D "/Game/SoundEffects/spacebar-click-keyboard-199448.spacebar-click-keyboard-199448" 0.2 0.5 0.1 0 0)
    (else
      (Utilities|FlowControl|FlipFlop
        (:A
          (Audio|PlaySound2D "/Game/SoundEffects/MS_door-open.MS_door-open" 0.3 1.0 0.0 0 0)
          (bind _doorfloat (Timeline|OpenDoorTimeline PlayFromStart)
            (:Update
              (Transformation|SetRelativeRotation (Variables|Default|GetDoor) (Math|Rotator|MakeRotator 0.0 0.0 (Math|Float|Lerp 0.0 -9e+01 _doorfloat)) false false))))
        (:B
          (Audio|PlaySound2D "/Game/SoundEffects/MS_door-close.MS_door-close" 0.3 1.0 0.0 0 0)
          (Timeline|OpenDoorTimeline Reverse))))))

(event Custom|CheckUpdateBatteryColour
  (bind _returnvalue (Actor|GetActorOfClass "/Game/Blueprints/BP_BatteryStorage.BP_BatteryStorage_C"))
  (if (>= (Variables|/Game/Blueprints/BP_BatteryStorage.BP_BatteryStorage_C|GetBatteriesCollected _returnvalue) (Variables|Default|GetBatteriesRequiredToUnlock))
    (Default|ChangeBatteryLightColour (Variables|Default|GetVaultBattery))))

(fn ConstructionScript)